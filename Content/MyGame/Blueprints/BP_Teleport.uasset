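; BP_Teleport is a paired teleporter actor that moves any actor overlapping its trigger boxes to a linked Exit teleporter.
; Each of the two boxes sends the actor to the opposite-numbered arrow on the Exit, keeping its rotation.
; Before teleporting, it calls ReloadLogic on the Exit, which briefly disables that teleporter to prevent an immediate bounce back.
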(event OnComponentBeginOverlap(Box)
  (params (OverlappedComponent :type Primitive%20Component%20Object%20Reference) (OtherActor :type Actor%20Object%20Reference) (OtherComp :type Primitive%20Component%20Object%20Reference) (OtherBodyIndex :type Integer) (bFromSweep :type Boolean) (SweepResult :type Hit%20Result%20Structure%20%28by%20ref%29))
  (if (Variables|Default|GetbAvailable)
    (bind _exit (Variables|Default|GetExit)
      (:then
        (CallFunction|ReloadLogic _exit)
        (Transformation|Teleport OtherActor (Transformation|GetWorldLocation (Variables|BP_Teleport_C|GetArrow1 _exit)) (Transformation|GetActorRotation OtherActor)))
      (:else))))

(event OnComponentBeginOverlap(Box1)
  (params (OverlappedComponent :type Primitive%20Component%20Object%20Reference) (OtherActor :type Actor%20Object%20Reference) (OtherComp :type Primitive%20Component%20Object%20Reference) (OtherBodyIndex :type Integer) (bFromSweep :type Boolean) (SweepResult :type Hit%20Result%20Structure%20%28by%20ref%29))
  (if (Variables|Default|GetbAvailable)
    (bind _exit (Variables|Default|GetExit)
      (:then
        (CallFunction|ReloadLogic _exit)
        (Transformation|Teleport OtherActor (Transformation|GetWorldLocation (Variables|BP_Teleport_C|GetArrow _exit)) (Transformation|GetActorRotation OtherActor)))
      (:else))))

(event Custom|ReloadLogic
  (Variables|Default|SetbAvailable false)
  (Utilities|FlowControl|Delay 2.0)
  (Variables|Default|SetbAvailable true))

(event Custom|TeleportLogic
  (params (Target :type Actor%20Object%20Reference)))

(event EventBeginPlay)

(event Collision|EventActorBeginOverlap
  (params (OtherActor :type Actor%20Object%20Reference)))

(event EventTick
  (params (DeltaSeconds :type Float%20%28single-precision%29)))

(fn ConstructionScript)