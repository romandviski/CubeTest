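; BP_TestActor is a sandbox actor demonstrating how C++ functions, events and variables appear in Blueprints, alongside Blueprint-declared functions.
; Its only live behavior is printing "Hello" from the C++ native event; BeginPlay, Tick and the implementable event are empty.
; Disconnected example snippets show callable versus pure calls, variable access and random-number pure nodes feeding prints.
; The Blueprint-declared functions are stubs, with the pure one returning zero.
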(event EventBeginPlay)

(event EventTick
  (params (DeltaSeconds :type Float%20%28single-precision%29)))

(event EventMyBlueprintImplementableEventFunction
  ;[0.5 0 0.5] Ивенты из плюсов
)

(event EventMyBlueprintNativeEventFunction
  ;[0.5 0 0.5] Ивенты из плюсов
  (Development|PrintString "Hello"))

(fn ConstructionScript)

(fn BlueprintFunction)

(fn BlueprintPureFunction
  (return 0))

(fn BlueprintFunctionCompact)